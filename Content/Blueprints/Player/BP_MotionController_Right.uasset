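; Right-hand VR motion controller Blueprint, a child class that sets its hand to Right and tracks which fingers touch objects for hand animation.
; The construction script assigns two collision components per finger to the parent's finger variables.
; Each component's begin-overlap event calls SetFlag, which marks that segment's slot in the TouchFlags array only while GripState is in one specific state.
; Nothing here clears the flags; the leftover clearing nodes are unconnected.
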(event OnComponentBeginOverlap(Thumb1Collision)
  (params (OverlappedComponent :type Primitive%20Component%20Object%20Reference) (OtherActor :type Actor%20Object%20Reference) (OtherComp :type Primitive%20Component%20Object%20Reference) (OtherBodyIndex :type Integer) (bFromSweep :type Boolean) (SweepResult :type Hit%20Result%20Structure%20%28by%20ref%29))
  ;[0 0.2657 0.3281] [BasicVR] Hand Anim. Record overlap state of fingers.
  (Utilities|SetFlag 6))

(event OnComponentBeginOverlap(Index1Collision)
  (params (OverlappedComponent :type Primitive%20Component%20Object%20Reference) (OtherActor :type Actor%20Object%20Reference) (OtherComp :type Primitive%20Component%20Object%20Reference) (OtherBodyIndex :type Integer) (bFromSweep :type Boolean) (SweepResult :type Hit%20Result%20Structure%20%28by%20ref%29))
  ;[0 0.2657 0.3281] [BasicVR] Hand Anim. Record overlap state of fingers.
  (Utilities|SetFlag 5))

(event OnComponentBeginOverlap(Pinky1Collision)
  (params (OverlappedComponent :type Primitive%20Component%20Object%20Reference) (OtherActor :type Actor%20Object%20Reference) (OtherComp :type Primitive%20Component%20Object%20Reference) (OtherBodyIndex :type Integer) (bFromSweep :type Boolean) (SweepResult :type Hit%20Result%20Structure%20%28by%20ref%29))
  ;[0 0.2657 0.3281] [BasicVR] Hand Anim. Record overlap state of fingers.
  (Utilities|SetFlag 9))

(event OnComponentBeginOverlap(Middle1Collision)
  (params (OverlappedComponent :type Primitive%20Component%20Object%20Reference) (OtherActor :type Actor%20Object%20Reference) (OtherComp :type Primitive%20Component%20Object%20Reference) (OtherBodyIndex :type Integer) (bFromSweep :type Boolean) (SweepResult :type Hit%20Result%20Structure%20%28by%20ref%29))
  ;[0 0.2657 0.3281] [BasicVR] Hand Anim. Record overlap state of fingers.
  (Utilities|SetFlag 7))

(event OnComponentBeginOverlap(Ring1Collision)
  (params (OverlappedComponent :type Primitive%20Component%20Object%20Reference) (OtherActor :type Actor%20Object%20Reference) (OtherComp :type Primitive%20Component%20Object%20Reference) (OtherBodyIndex :type Integer) (bFromSweep :type Boolean) (SweepResult :type Hit%20Result%20Structure%20%28by%20ref%29))
  ;[0 0.2657 0.3281] [BasicVR] Hand Anim. Record overlap state of fingers.
  (Utilities|SetFlag 8))

(event OnComponentBeginOverlap(Index2Collision)
  (params (OverlappedComponent :type Primitive%20Component%20Object%20Reference) (OtherActor :type Actor%20Object%20Reference) (OtherComp :type Primitive%20Component%20Object%20Reference) (OtherBodyIndex :type Integer) (bFromSweep :type Boolean) (SweepResult :type Hit%20Result%20Structure%20%28by%20ref%29))
  ;[0 0.2657 0.3281] [BasicVR] Hand Anim. Record overlap state of fingers.
  (Utilities|SetFlag))

(event OnComponentBeginOverlap(Middle2Collision)
  (params (OverlappedComponent :type Primitive%20Component%20Object%20Reference) (OtherActor :type Actor%20Object%20Reference) (OtherComp :type Primitive%20Component%20Object%20Reference) (OtherBodyIndex :type Integer) (bFromSweep :type Boolean) (SweepResult :type Hit%20Result%20Structure%20%28by%20ref%29))
  ;[0 0.2657 0.3281] [BasicVR] Hand Anim. Record overlap state of fingers.
  (Utilities|SetFlag 2))

(event OnComponentBeginOverlap(Ring2Collision)
  (params (OverlappedComponent :type Primitive%20Component%20Object%20Reference) (OtherActor :type Actor%20Object%20Reference) (OtherComp :type Primitive%20Component%20Object%20Reference) (OtherBodyIndex :type Integer) (bFromSweep :type Boolean) (SweepResult :type Hit%20Result%20Structure%20%28by%20ref%29))
  ;[0 0.2657 0.3281] [BasicVR] Hand Anim. Record overlap state of fingers.
  (Utilities|SetFlag 3))

(event OnComponentBeginOverlap(Thumb2Collision)
  (params (OverlappedComponent :type Primitive%20Component%20Object%20Reference) (OtherActor :type Actor%20Object%20Reference) (OtherComp :type Primitive%20Component%20Object%20Reference) (OtherBodyIndex :type Integer) (bFromSweep :type Boolean) (SweepResult :type Hit%20Result%20Structure%20%28by%20ref%29))
  ;[0 0.2657 0.3281] [BasicVR] Hand Anim. Record overlap state of fingers.
  (Utilities|SetFlag 1))

(event OnComponentBeginOverlap(Pinky2Collision)
  (params (OverlappedComponent :type Primitive%20Component%20Object%20Reference) (OtherActor :type Actor%20Object%20Reference) (OtherComp :type Primitive%20Component%20Object%20Reference) (OtherBodyIndex :type Integer) (bFromSweep :type Boolean) (SweepResult :type Hit%20Result%20Structure%20%28by%20ref%29))
  ;[0 0.2657 0.3281] [BasicVR] Hand Anim. Record overlap state of fingers.
  (Utilities|SetFlag 4))

(event EventBeginPlay
  (|CallParentFunction)
  (Variables|Default|SetHand "Right"))

(event EventTick
  (params (DeltaSeconds :type Float%20%28single-precision%29))
  (|CallParentFunction DeltaSeconds) ; This node is disabled and will not be called.\nDrag off pins to build functionality.
)

(fn ConstructionScript
  (|CallParentFunction)
  (Utilities|FlowControl|Sequence
    (:then_0
      (Variables|Default|SetThumb1 (Variables|Default|GetThumb1Collision)))
    (:then_1
      (Variables|Default|SetThumb2 (Variables|Default|GetThumb2Collision)))
    (:then_2
      (Variables|Default|SetPinky1 (Variables|Default|GetPinky1Collision)))
    (:then_3
      (Variables|Default|SetPinky2 (Variables|Default|GetPinky2Collision)))
    (:then_4
      (Variables|Default|SetRing1 (Variables|Default|GetRing1Collision)))
    (:then_5
      (Variables|Default|SetRing2 (Variables|Default|GetRing2Collision)))
    (:then_6
      (Variables|Default|SetMiddle1 (Variables|Default|GetMiddle1Collision)))
    (:then_7
      (Variables|Default|SetMiddle2 (Variables|Default|GetMiddle2Collision)))
    (:then_8
      (Variables|Default|SetIndex1 (Variables|Default|GetIndex1Collision)))
    (:then_9
      (Variables|Default|SetIndex2 (Variables|Default|GetIndex2Collision)))))