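; BP_Button is a physical push button for VR motion controllers that glows when fully pressed.
; An overlapping controller starts tracking, and Tick projects its hand movement onto the button's up axis, pushing the button in up to MaximumTravel.
; A full press swaps the material, waits briefly, then interpolates back and restores it.
; A partial press stays where released, as only a full press triggers the return.
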(event OnComponentEndOverlap(Button)
  (params (OverlappedComponent :type Primitive%20Component%20Object%20Reference) (OtherActor :type Actor%20Object%20Reference) (OtherComp :type Primitive%20Component%20Object%20Reference) (OtherBodyIndex :type Integer))
  (bind _asbp_motion_controller_base (Utilities|Casting|CastToBP_MotionController_Base OtherActor))
  (if (== _asbp_motion_controller_base (Variables|Default|GetCurrentMotionController))
    (Variables|Default|SetIsTracking false)
    (Variables|Default|SetCurrentMotionController 0)))

(event OnComponentBeginOverlap(Button)
  (params (OverlappedComponent :type Primitive%20Component%20Object%20Reference) (OtherActor :type Actor%20Object%20Reference) (OtherComp :type Primitive%20Component%20Object%20Reference) (OtherBodyIndex :type Integer) (bFromSweep :type Boolean) (SweepResult :type Hit%20Result%20Structure%20%28by%20ref%29))
  (if (Math|Boolean|ANDBoolean (not (Variables|Default|GetIsTracking)) (not (Variables|Default|GetIsReturning)) (not (Variables|Default|GetIsFullyPressed)))
    (bind _asbp_motion_controller_base (Utilities|Casting|CastToBP_MotionController_Base OtherActor))
    (Variables|Default|SetCurrentMotionController _asbp_motion_controller_base)
    (Variables|Default|SetIsTracking true)
    (Variables|Default|SetInitialMCLocation (Transformation|GetWorldLocation (Variables|/Game/Blueprints/Player/BP_MotionController_Base.BP_MotionController_Base_C|GetHandMesh _asbp_motion_controller_base)))
    (Variables|Default|SetInitialButtonLocation (Transformation|GetWorldLocation (Variables|Default|GetButton)))))

(event Custom|FullyPressed
  (Rendering|Material|SetMaterial (Variables|Default|GetButton) 0 "/Game/Assets/Laser/M_Glow.M_Glow")
  (Variables|Default|SetIsTracking false)
  (Variables|Default|SetIsFullyPressed true)
  (Utilities|FlowControl|Delay 1.0)
  (Variables|Default|SetIsReturning true))

(event Custom|TrachMC
  (Variables|Default|SetCurrentTravel (Math|Float|Clamp(Float) (Math|Float|Absolute(Float) (Math|Vector|VectorLength (Math|Vector|ProjectVectorontoVector (- (Transformation|GetWorldLocation (Variables|/Game/Blueprints/Player/BP_MotionController_Base.BP_MotionController_Base_C|GetHandMesh (Variables|Default|GetCurrentMotionController))) (Variables|Default|GetInitialMCLocation)) (Math|Vector|GetUpVector (Variables|Default|GetButton))))) 0.0 (Variables|Default|GetMaximumTravel)))
  (bind _output_get (Variables|Default|SetButtonCurrentLocation (- (Variables|Default|GetInitialButtonLocation) (* (Math|Vector|GetUpVector (Variables|Default|GetButton)) (Variables|Default|GetCurrentTravel)))))
  (Transformation|SetWorldLocation (Variables|Default|GetButton) _output_get false false)
  (if (>= (Variables|Default|GetCurrentTravel) (Variables|Default|GetMaximumTravel))
    (CallFunction|FullyPressed)))

(event Custom|ReturnToPosition
  (bind _output_get (Variables|Default|SetButtonCurrentLocation (Math|Interpolation|VInterpTo (Variables|Default|GetButtonCurrentLocation) (Variables|Default|GetInitialButtonLocation) (Utilities|Time|GetWorldDeltaSeconds) 5.0)))
  (Transformation|SetWorldLocation (Variables|Default|GetButton) _output_get false false)
  (if (Math|Vector|Equal(Vector) (Variables|Default|GetButtonCurrentLocation) (Variables|Default|GetInitialButtonLocation) 0.0001)
    (CallFunction|FullyReturned)))

(event Custom|FullyReturned
  (Variables|Default|SetIsReturning false)
  (Variables|Default|SetIsFullyPressed false)
  (Rendering|Material|SetMaterial (Variables|Default|GetButton) 0 "/Game/Assets/Meshes/Materials/MI_SmallCubes.MI_SmallCubes"))

(event EventBeginPlay)

(event Collision|EventActorBeginOverlap
  (params (OtherActor :type Actor%20Object%20Reference)))

(event EventTick
  (params (DeltaSeconds :type Float%20%28single-precision%29))
  (if (Variables|Default|GetIsTracking)
    (CallFunction|TrachMC)
    (elif (Variables|Default|GetIsReturning)
      (CallFunction|ReturntoPosition))))

(fn ConstructionScript)