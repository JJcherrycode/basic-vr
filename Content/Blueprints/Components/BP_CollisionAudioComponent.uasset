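; Actor component that plays collision impact sounds for its owner, configured by a row in DT_AudioImpact.
; It binds to hits on tagged primitive components, falling back to actor hits when none are tagged.
; Hits are filtered by impulse threshold, cooldown, play flags, and transform change or time since the last rejected hit.
; Normalized impulse selects the heavy sound or modulates the default sound's pitch and volume.
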(event Custom|Event%20On%20Impact
  (params (Impulse :type Vector) (Hit :type Hit%20Result%20Structure))
  (bind _location (Collision|BreakHitResult Hit))
  ;[1 1 1] Simple component to manage playing sounds when collision impacts are received
  ;;[1 1 1] Also set Impulse Maginitude
  (bind _valid (CallFunction|DetectValidHit Impulse))
  (if _valid
    ;;[1 1 1] Normalise Impulse Maginitude between TresholdMin and Max, stores in the same variable
    (CallFunction|NormalizeImpulse)
    (CallFunction|PlayImpactSound _location)
    (CallFunction|RecordTrigger (Transformation|GetActorTransform (Components|GetOwner)))
    (Variables|Default|SetbFirstHit false)
    (Default|CallOnPlay)
    (if (Variables|Default|GetbIsDebugLogEnabled)
      (Rendering|Debug|DrawDebugString _location (Utilities|String|Append "Collision Impulse Magnitude: " (Utilities|String|ToString(Float) (Variables|Default|GetImpulseMagnitude)) " (" (Utilities|String|ToString(Float) (Math|Vector|VectorLength Impulse)) ")") 0 "(R=1.000000,G=1.000000,B=1.000000,A=1.000000)" 3.0))))

(event Custom|Initialize
  ;[1 1 1] Simple component to manage playing sounds when collision impacts are received
  (bind _returnvalue (Utilities|GetDataTableRow "/Game/Audio/Data/DT_AudioImpact.DT_AudioImpact" (Variables|Default|GetImpactNameRef))
    (:then
      (Variables|Default|SetImpactDataNew _returnvalue)
      (CallFunction|BindtoCollisionEvents))))

(event Custom|Set%20Impact%20Name%20Ref
  (params (Name%20Ref :type Name))
  ;[1 1 1] Simple component to manage playing sounds when collision impacts are received
  (Variables|Default|SetImpactNameRef Name%20Ref)
  (CallFunction|Initialize))

(event Custom|OnTaggedComponentHit
  (params (HitComponent :type Primitive%20Component%20Object%20Reference) (OtherActor :type Actor%20Object%20Reference) (OtherComp :type Primitive%20Component%20Object%20Reference) (NormalImpulse :type Vector) (Hit :type Hit%20Result%20Structure%20%28by%20ref%29))
  ;[1 1 1] Simple component to manage playing sounds when collision impacts are received
  (CallFunction|EventonImpact NormalImpulse Hit))

(event Custom|OnActorHit
  (params (SelfActor :type Actor%20Object%20Reference) (OtherActor :type Actor%20Object%20Reference) (NormalImpulse :type Vector) (Hit :type Hit%20Result%20Structure%20%28by%20ref%29))
  ;[1 1 1] Simple component to manage playing sounds when collision impacts are received
  (CallFunction|EventonImpact NormalImpulse Hit))

(event Custom|Bind%20To%20Collision%20Events
  (bind _returnvalue (Components|GetOwner))
  (bind _collisioncomponenttag (Variables|Default|GetCollisionComponentTag))
  (bind _returnvalue_2 (Actor|GetComponentsbyTag _returnvalue "/Script/Engine.PrimitiveComponent" _collisioncomponenttag))
  ;[1 1 1] Bind to collision events. Will listen on collision of owner actor components tagged with CollisionComponentTag or to collision of actor
  (Utilities|IsValid _returnvalue
    (:Is%20Valid
      (if (!= (Utilities|Array|Length _returnvalue_2) 0)
        (for _array_element _returnvalue_2
          (Collision|BindEventtoOnComponentHit _array_element (EventDispatchers|CreateEvent :!event Custom|OnTaggedComponentHit)))
        (else
          (Collision|BindEventtoOnActorHit (Components|GetOwner) (EventDispatchers|CreateEvent :!event Custom|OnActorHit)))))))

(event EventBeginPlay
  ;[1 1 1] Simple component to manage playing sounds when collision impacts are received
  (CallFunction|Initialize))

(fn SetCanPlay
  (params (Can%20Play :type Boolean))
  (Variables|Default|SetbCanPlay Can%20Play)
  (Variables|Default|SetLastTriggerTransform (Transformation|GetActorTransform (Components|GetOwner)))
  (Variables|Default|SetbFirstHit true))

(fn NormalizeImpulse
  (bind _impactdatanew (Variables|Default|GetImpactDataNew))
  (bind (_impactmagnitudetresholdmin _impactmagnitudetresholdmax) (Utilities|Struct|BreakS_AudioImpactData _impactdatanew))
  (Variables|Default|SetImpulseMagnitude (Math|Float|MapRangeClamped (Variables|Default|GetImpulseMagnitude) _impactmagnitudetresholdmin _impactmagnitudetresholdmax 0.0 1.0)))

(fn DetectValidHit
  (params (Impulse :type Vector))
  (bind _impactdatanew (Variables|Default|GetImpactDataNew))
  (bind (_retriggercooldown _impactmagnitudetresholdmin) (Utilities|Struct|BreakS_AudioImpactData _impactdatanew))
  (Variables|Default|SetImpulseMagnitude (Math|Vector|VectorLength Impulse))
  (if (Math|Boolean|ANDBoolean (>= (- (Utilities|Time|GetGameTimeinSeconds) (Variables|Default|GetLastTriggerGameTime)) _retriggercooldown) (>= (Variables|Default|GetImpulseMagnitude) _impactmagnitudetresholdmin) (Variables|Default|GetbCanPlay) (Variables|Default|GetbCanEverPlay) (Math|Boolean|ORBoolean (not (Class|KismetMathLibrary|NearlyEqualTransformTransform (Variables|Default|GetLastTriggerTransform) (Transformation|GetActorTransform (Components|GetOwner)) (Variables|Default|GetTriggerLocationDeltaThreshold) (Variables|Default|GetTriggerRotationDeltaThreshold) 0.0001)) (Variables|Default|GetbFirstHit) (Variables|Default|GetbDisableDeltaThreshold) (>= (- (Utilities|Time|GetGameTimeinSeconds) (Variables|Default|GetLastInvalidHitGameTime)) 0.1)))
    (return true)
    (else
      (Variables|Default|SetLastInvalidHitGameTime (Utilities|Time|GetGameTimeinSeconds))
      (return false))))

(fn PlayImpactSound
  (params (Location :type Vector))
  (bind _impactdatanew (Variables|Default|GetImpactDataNew))
  (bind (_pitchmodulationmin _pitchmodulationmax _volumemodulationmin _volumemodulationmax) (Utilities|Struct|BreakS_AudioImpactData _impactdatanew))
  (Utilities|FlowControl|Sequence
    (:then_0
      (if (>= (Variables|Default|GetImpulseMagnitude) 1.0)
        ;[1 1 1] Magnitude >= TresholdMax? Play "heavy hit" sound as is
        (LocalVariables|SetSound (Utilities|Struct|BreakS_AudioImpactData (Variables|Default|GetImpactDataNew)))
        (else
          ;[1 1 1] Magnitude< TresholdMax: play "Light Hit" sound with amplitude and pitch adjusted
          (LocalVariables|SetPitch (Math|Float|MapRangeClamped (Variables|Default|GetImpulseMagnitude) 0.0 1.0 _pitchmodulationmin _pitchmodulationmax))
          (LocalVariables|SetVolume (Math|Float|MapRangeClamped (Variables|Default|GetImpulseMagnitude) 0.0 1.0 _volumemodulationmin _volumemodulationmax))
          (LocalVariables|SetSound (Utilities|Struct|BreakS_AudioImpactData (Variables|Default|GetImpactDataNew))))))
    (:then_1
      (Audio|PlaySoundatLocation (LocalVariables|GetSound) Location "0, 0, 0" (LocalVariables|GetVolume) (LocalVariables|GetPitch) 0.0 0 0 0))))

(fn SetCanEverPlay
  (params (Can%20Ever%20Play :type Boolean))
  (bind _output_get (Variables|Default|SetbCanEverPlay Can%20Ever%20Play))
  (if _output_get
    (Variables|Default|SetbFirstHit true)))

(fn RecordTrigger
  (params (LastTriggerTransform :type Transform))
  (Variables|Default|SetLastTriggerGameTime (Utilities|Time|GetGameTimeinSeconds))
  (Variables|Default|SetLastTriggerTransform LastTriggerTransform))

(fn SetDisableDeltaThreshold
  (params (bDisableDeltaThreshold :type Boolean))
  (Variables|Default|SetbDisableDeltaThreshold bDisableDeltaThreshold))