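; BP_Katana is a katana that the player can pick up and drop with a VR motion controller.
; Pickup switches the mesh's collision type to Pawn, attaches the actor to the hand mesh and aligns it to KatanaSocket.
; Drop switches to a custom collision channel, detaches and applies the captured velocity as a force.
; BeginPlay enables physical collision sounds through CollisionAudioComponent.
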(event EventBeginPlay
  ;[1 0.4927 0.02567] [BasicVR] Physical collision sound
  (Default|SetCanPlay (Variables|Default|GetCollisionAudioComponent) true))

(event EventTick
  (params (DeltaSeconds :type Float%20%28single-precision%29)))

(event EventPickup
  (params (Constraint :type Physics%20Constraint%20Component%20Object%20Reference) (HandMesh :type Skeletal%20Mesh%20Component%20Object%20Reference))
  (bind _returnvalue (VehicleSound|GetRootComponent))
  (Collision|SetCollisionObjectType (Variables|Debug|GetStaticMeshComponent) "ECC_Pawn")
  (Transformation|AttachComponentToComponent _returnvalue HandMesh "" "SnapToTarget" "SnapToTarget" "KeepWorld" true)
  (Transformation|SetWorldTransform _returnvalue (Transformation|GetSocketTransform HandMesh "KatanaSocket" "RTS_World") false false))

(event EventDrop
  (params (Constraint :type Physics%20Constraint%20Component%20Object%20Reference))
  (Variables|Default|SetCurVelocity (Transformation|GetVelocity))
  (Collision|SetCollisionObjectType (Variables|Debug|GetStaticMeshComponent) "ECC_GameTraceChannel2")
  (Transformation|DetachFromActor "KeepWorld" "KeepWorld" "KeepWorld")
  (Physics|AddForce (Variables|Debug|GetStaticMeshComponent) (Variables|Default|GetCurVelocity) "None" false))

(fn ConstructionScript)